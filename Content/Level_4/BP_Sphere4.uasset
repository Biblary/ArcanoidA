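; BP_Sphere4 is a bouncing ball actor in Level 4 that is destroyed when it overlaps a kill Z volume.
; Each tick it sweeps along Direction at Speed in the XY plane and mirrors Direction off the surface normal on a blocking hit.
; Overlapping a KillZVolume fires CallCallDBD, destroys the ball and plays a 2D sound.
; Leftover cube-scoring and speed-increase logic is disconnected and never runs.
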(event EventBeginPlay)

(event EventTick
  (params (DeltaSeconds :type Float%20%28single-precision%29))
  (bind _sweephitresult (Transformation|AddActorWorldOffset (Math|Vector|MakeVector (.x (* (* (Variables|Default|GetDirection) (Variables|Default|Getspeed)) DeltaSeconds)) (.y (* (* (Variables|Default|GetDirection) (Variables|Default|Getspeed)) DeltaSeconds)) 0.0) true))
  (if (.bBlockingHit (Collision|BreakHitResult _sweephitresult))
    (Variables|Default|SetDirection (Math|Vector|GetReflectionVector (Variables|Default|GetDirection) (.Normal (Collision|BreakHitResult _sweephitresult))))))

(event Collision|EventActorBeginOverlap
  (params (OtherActor :type Actor%20Object%20Reference))
  (Utilities|Casting|CastToKillZVolume OtherActor)
  (Default|CallCallDBD)
  (Actor|DestroyActor)
  (Audio|PlaySound2D "/Engine/VREditor/Sounds/UI/Foliage_Placed.Foliage_Placed" 1.0 1.0 0.0 0 0))

(event Collision|EventHit
  (params (MyComp :type Primitive%20Component%20Object%20Reference) (Other :type Actor%20Object%20Reference) (OtherComp :type Primitive%20Component%20Object%20Reference) (bSelfMoved :type Boolean) (HitLocation :type Vector :default "0, 0, 0") (HitNormal :type Vector :default "0, 0, 0") (NormalImpulse :type Vector :default "0, 0, 0") (Hit :type Hit%20Result%20Structure%20%28by%20ref%29)))

(fn ConstructionScript)