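; Child sphere Blueprint in the Level_10 folder that inherits its active behavior from its parent class.
; BeginPlay and the construction script only call the parent, while the overlap and Tick events are disabled placeholders.
; A disconnected, never-executed chain would step the sphere through timed material changes, spawn BP_BOOOM at its transform, then destroy the actor.
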(event EventBeginPlay
  (|CallParentFunction))

(event Collision|EventActorBeginOverlap
  (params (OtherActor :type Actor%20Object%20Reference))
  (|CallParentFunction OtherActor) ; Этот узел отключен и не будет вызываться.\nПеретащите контакты, чтобы построить функционал.
)

(event EventTick
  (params (DeltaSeconds :type Float%20%28single-precision%29))
  (|CallParentFunction DeltaSeconds) ; Этот узел отключен и не будет вызываться.\nПеретащите контакты, чтобы построить функционал.
)

(fn ConstructionScript
  (|CallParentFunction))