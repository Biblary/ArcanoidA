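; BP_Cube_Child10 is a Level 10 cube Blueprint, derived from a parent class, that randomly changes its material during play.
; BeginPlay starts a looping two-second timer that calls the RGB event.
; RGB uses nested random booleans to apply one of four materials to slot 0 of the Cube component, with equal odds.
; Overlap and Tick events are disabled stubs, and the construction script only calls the parent.
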(event Custom|RGB
  (bind _cube (Variables|Default|GetCube))
  (bind _cube_2 (Variables|Default|GetCube))
  (if (Math|Random|RandomBool)
    (if (Math|Random|RandomBool)
      (Utilities|IsValid _cube_2
        (:Is%20Valid
          (Rendering|Material|SetMaterial _cube_2 0 "/Game/Level_5/NewMaterial3.NewMaterial3")))
      (else
        (Utilities|IsValid _cube_2
          (:Is%20Valid
            (Rendering|Material|SetMaterial _cube_2 0 "/Game/Level_5/NewMaterial5.NewMaterial5")))))
    (elif (Math|Random|RandomBool)
      (Utilities|IsValid _cube
        (:Is%20Valid
          (Rendering|Material|SetMaterial (Variables|Default|GetCube) 0 "/Game/Level_5/NewMaterial4.NewMaterial4")))
      (else
        (Utilities|IsValid _cube
          (:Is%20Valid
            (Rendering|Material|SetMaterial _cube 0 "/Game/Level_5/NewMaterial6.NewMaterial6")))))))

(event EventBeginPlay
  (Utilities|Time|SetTimerbyEvent (delegate Custom|RGB) 2.0 true))

(event Collision|EventActorBeginOverlap
  (params (OtherActor :type Actor%20Object%20Reference))
  (|CallParentFunction OtherActor) ; Этот узел отключен и не будет вызываться.\nПеретащите контакты, чтобы построить функционал.
)

(event EventTick
  (params (DeltaSeconds :type Float%20%28single-precision%29)))

(fn ConstructionScript
  (|CallParentFunction))