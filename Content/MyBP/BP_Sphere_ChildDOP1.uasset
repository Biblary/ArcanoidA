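; BP_Sphere_ChildDOP1 is a child sphere Blueprint that acts as a timed fuse, ending in the spawn of BP_BOOOM.
; After the parent BeginPlay runs, a chain of Delay nodes steps the Sphere through three materials over several seconds.
; It then spawns BP_BOOOM at its own transform and destroys itself, while the construction script only calls the parent.
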(event EventBeginPlay
  (|CallParentFunction)
  (Utilities|FlowControl|Delay 3.0)
  (Rendering|Material|SetMaterial (Variables|Default|GetSphere) 0 "/Game/CubeAndTexture/NewMaterial6.NewMaterial6")
  (Utilities|FlowControl|Delay 2.0)
  (Rendering|Material|SetMaterial (Variables|Default|GetSphere) 0 "/Game/CubeAndTexture/NewMaterial7.NewMaterial7")
  (Utilities|FlowControl|Delay 2.0)
  (Rendering|Material|SetMaterial (Variables|Default|GetSphere) 0 "/Game/CubeAndTexture/NewMaterial8.NewMaterial8")
  (Utilities|FlowControl|Delay 1.0)
  (Game|SpawnActorfromClass "/Game/MyBP/BP_BOOOM.BP_BOOOM_C" (Transformation|GetActorTransform) "Undefined" "MultiplyWithRoot" 0 0)
  (Actor|DestroyActor))

(event Collision|EventActorBeginOverlap
  (params (OtherActor :type Actor%20Object%20Reference))
  (|CallParentFunction OtherActor) ; Этот узел отключен и не будет вызываться.\nПеретащите контакты, чтобы построить функционал.
)

(event EventTick
  (params (DeltaSeconds :type Float%20%28single-precision%29))
  (|CallParentFunction DeltaSeconds) ; Этот узел отключен и не будет вызываться.\nПеретащите контакты, чтобы построить функционал.
)

(fn ConstructionScript
  (|CallParentFunction))