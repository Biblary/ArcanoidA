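; Player paddle pawn for what appears to be a Breakout-style ball game, sliding sideways with swept offsets and handling score, lives, pause and end screens.
; It spawns BP_Sphere balls and binds their DBD event, which costs HP and either respawns a ball or shows game over.
; AddedScore raises the score, notifies listeners and shows the win screen above a threshold.
; Bracket keys act as debug shortcuts for score and an extra sphere.
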(event Custom|DBD_event
  (bind _result (Math|Integer|DecrementInt (Variables|Default|GetHP))
    (:%20%20
      (if (<= _result 0)
        (bind _returnvalue (UserInterface|CreateWidget (Variables|Default|GetgameOverBWP)))
        (UserInterface|Viewport|AddtoViewport _returnvalue 0)
        (Variables|/Script/Engine.PlayerController|SetbShowMouseCursor (Game|GetPlayerController 0) true)
        (Game|SetGamePaused true)
        (else
          (bind _returnvalue_2 (Game|SpawnActorfromClass "/Game/MyBP/BP_Sphere.BP_Sphere_C" (Math|Transform|MakeTransform (Transformation|GetWorldLocation (Variables|Default|GetCapsule)) "0, 0, 0" "1.000000,1.000000,1.000000") "AlwaysSpawn" "SelectDefaultAtRuntime" 0 0))
          (bind _output_get (Variables|Default|SetSphere _returnvalue_2))
          (EventDispatchers|BindEventtoCallDBD _output_get (delegate Custom|DBD_event)))))))

(event Custom|GG
  (if (not (<= (Variables|Default|GetAllScore) (Variables|Default|GetNedScoreWin)))
    (Game|SetGamePaused true)
    (bind _returnvalue (UserInterface|CreateWidget (Variables|Default|GetGGWP)))
    (UserInterface|Viewport|AddtoViewport _returnvalue 0)
    (Variables|/Script/Engine.PlayerController|SetbShowMouseCursor (Game|GetPlayerController 0) true)
    (Widget|RemovefromParent (stale EventBeginPlay _returnvalue_2))))

(event EventBeginPlay
  (bind _returnvalue (UserInterface|CreateWidget "/Game/Wiget/BWP_space.BWP_space_C"))
  (UserInterface|Viewport|AddtoViewport _returnvalue 0)
  (bind _returnvalue_2 (UserInterface|CreateWidget "/Game/Wiget/WogetGame/BPW_Helper.BPW_Helper_C"))
  (UserInterface|Viewport|AddtoViewport _returnvalue_2 0)
  (if (not (Variables|Default|GetSpawn%20or\no%20Spawn))
    (Variables|Default|SetSpawn%20or\no%20Spawn false)
    (bind _returnvalue_3 (Game|SpawnActorfromClass "/Game/MyBP/BP_Sphere.BP_Sphere_C" (Math|Transform|MakeTransform (Transformation|GetWorldLocation (Variables|Default|GetCapsule)) "0, 0, 0" "1.000000,1.000000,1.000000") "AlwaysSpawn" "SelectDefaultAtRuntime" 0 0))
    (bind _output_get (Variables|Default|SetSphere _returnvalue_3))
    (EventDispatchers|BindEventtoCallDBD _output_get (delegate Custom|DBD_event))))

(event Collision|EventActorBeginOverlap
  (params (OtherActor :type Actor%20Object%20Reference)))

(event EventTick
  (params (DeltaSeconds :type Float%20%28single-precision%29)))

(event Collision|EventHit
  (params (MyComp :type Primitive%20Component%20Object%20Reference) (Other :type Actor%20Object%20Reference) (OtherComp :type Primitive%20Component%20Object%20Reference) (bSelfMoved :type Boolean) (HitLocation :type Vector :default "0, 0, 0") (HitNormal :type Vector :default "0, 0, 0") (NormalImpulse :type Vector :default "0, 0, 0") (Hit :type Hit%20Result%20Structure%20%28by%20ref%29))
  (Utilities|Casting|CastToBP_Sphere Other)
  (Audio|PlaySound2D "/Engine/VREditor/Sounds/UI/Drop_Item_From_ContentBrowser.Drop_Item_From_ContentBrowser" 1.0 1.0 0.0 0 0))

(event Input|ActionEvents|InputActionPause
  (params (Key :type Key%20Structure :default "None"))
  (:Pressed
    (if (Variables|Default|GetPauseON\OFF)
      (Variables|Default|SetPauseON\OFF false)
      (Game|SetGamePaused true)
      (bind _returnvalue (UserInterface|CreateWidget "/Game/Wiget/MenuWiget/PauseBP.PauseBP_C"))
      (UserInterface|Viewport|AddtoViewport _returnvalue 0)
      (Variables|/Script/Engine.PlayerController|SetbShowMouseCursor (Game|GetPlayerController 0) true)
      (else
        (Variables|Default|SetPauseON\OFF true)
        (Game|SetGamePaused false)
        (Widget|RemovefromParent _returnvalue)
        (Variables|/Script/Engine.PlayerController|SetbShowMouseCursor (Game|GetPlayerController 0) false)))))

(event Input|AxisEvents|InputAxisa\d
  (params (AxisValue :type Float%20%28single-precision%29))
  (if (< AxisValue 0.0)
    (bind _sweephitresult (Transformation|AddActorWorldOffset "0,-50.000000, 0" true))
    (if (.bBlockingHit (Collision|BreakHitResult _sweephitresult))
      _)))

(event Input|AxisEvents|InputAxisa\d
  (params (AxisValue :type Float%20%28single-precision%29))
  (if (> AxisValue 0.0)
    (bind _sweephitresult (Transformation|AddActorWorldOffset "0,50.000000,0.000000" true))
    (if (.bBlockingHit (Collision|BreakHitResult _sweephitresult))
      _)))

(event Input|KeyboardEvents|RightBracket
  (params (Key :type Key%20Structure :default "None"))
  (:Pressed
    (Game|SpawnActorfromClass "/Game/MyBP/BP_Sphere_ChildDOP1.BP_Sphere_ChildDOP1_C" (Math|Transform|MakeTransform (Transformation|GetWorldLocation (Variables|Default|GetCapsule)) "0, 0, 0" "1.000000,1.000000,1.000000") "AlwaysSpawn" "SelectDefaultAtRuntime" 0 0)))

(event Input|KeyboardEvents|LeftBracket
  (params (Key :type Key%20Structure :default "None"))
  (:Pressed
    (Variables|Default|SetAllScore (+ (Variables|Default|GetAddSocerCheat) 200))))

(event Input|KeyboardEvents|SpaceBar
  (params (Key :type Key%20Structure :default "None"))
  (:Pressed
    (Widget|RemovefromParent (stale EventBeginPlay _returnvalue))
    (if (Variables|Default|GetSpawn%20or\no%20Spawn)
      (Variables|Default|SetSpawn%20or\no%20Spawn false)
      (bind _returnvalue (Game|SpawnActorfromClass "/Game/MyBP/BP_Sphere.BP_Sphere_C" (Math|Transform|MakeTransform (Transformation|GetWorldLocation (Variables|Default|GetCapsule)) "0, 0, 0" "1.000000,1.000000,1.000000") "AlwaysSpawn" "SelectDefaultAtRuntime" 0 0))
      (bind _output_get (Variables|Default|SetSphere _returnvalue))
      (EventDispatchers|BindEventtoCallDBD _output_get (delegate Custom|DBD_event)))))

(fn ConstructionScript)

(fn AddedScore
  (params (Amount :type Integer))
  (Variables|Default|SetAllScore (+ (Variables|Default|GetAllScore) (Math|Integer|Absolute(Integer) Amount)))
  (Default|CallScoreChange)
  (CallFunction|GG))