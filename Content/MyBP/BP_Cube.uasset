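; BP_Cube is a breakable cube target that loses HP when hit by a BP_Sphere and awards score when destroyed.
; A hit at zero HP randomly either spawns an enlarged BP_Sphere_ChildDOP1 or just plays a click, each outcome having its own sound.
; It then calls CuveDead with the score and destroys the hit component rather than the actor.
; Sphere overlaps also set the cube's material slot, with no material specified.
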(event Custom|DesScoreCube)

(event Collision|EventActorBeginOverlap
  (params (OtherActor :type Actor%20Object%20Reference))
  (Utilities|Casting|CastToBP_Sphere OtherActor)
  (Rendering|Material|SetMaterial (Variables|Default|GetCube) 0 0))

(event Collision|EventHit
  (params (MyComp :type Primitive%20Component%20Object%20Reference) (Other :type Actor%20Object%20Reference) (OtherComp :type Primitive%20Component%20Object%20Reference) (bSelfMoved :type Boolean) (HitLocation :type Vector :default "0, 0, 0") (HitNormal :type Vector :default "0, 0, 0") (NormalImpulse :type Vector :default "0, 0, 0") (Hit :type Hit%20Result%20Structure%20%28by%20ref%29))
  (Utilities|Casting|CastToBP_Sphere Other)
  (if (<= (Variables|Default|GetHP) 0.0)
    (if (Math|Random|RandomBoolwithWeight 0.4)
      (Game|SpawnActorfromClass "/Game/MyBP/BP_Sphere_ChildDOP1.BP_Sphere_ChildDOP1_C" (Math|Transform|MakeTransform (Transformation|GetActorLocation) "0, 0, 0" "5.000000,5.000000,5.000000") "Undefined" "MultiplyWithRoot" 0 0)
      (Audio|PlaySound2D "/Engine/VREditor/Sounds/UI/Dockable_Window_Open.Dockable_Window_Open" 1.0 1.0 0.0 0 0)
      (else
        (Audio|PlaySound2D "/Engine/VREditor/Sounds/UI/Click_on_Button.Click_on_Button" 1.0 1.0 0.0 0 0)))
    (bind _output_get (Variables|Default|SetScore 1))
    (Default|CallCuveDead _output_get)
    (Components|DestroyComponent MyComp)
    (else
      (Variables|Default|SetHP (- (Variables|Default|GetHP) 1.0)))))

(fn ConstructionScript)