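; BP_Smok is an actor that stages a one-off timed explosion event and then reveals its own particle system, likely smoke.
; On BeginPlay it waits a random 40 to 60 seconds, plays a 2D explosion sound and spawns four BP_BOOOM actors at hardcoded corner positions.
; One second later it makes the particle system visible.
; A delayed self-destroy is left unconnected, so the actor never removes itself.
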(event EventBeginPlay
  (Utilities|FlowControl|Delay (Math|Random|RandomFloatinRange 4e+01 6e+01))
  (Audio|PlaySound2D "/Game/StarterContent/Audio/Explosion01.Explosion01" 1.0 1.0 0.0 0 0)
  (Game|SpawnActorfromClass "/Game/MyBP/BP_BOOOM.BP_BOOOM_C" (Math|Transform|MakeTransform "-130.000000,2840.000000,100.000000") "Undefined" "MultiplyWithRoot" 0 0)
  (Game|SpawnActorfromClass "/Game/MyBP/BP_BOOOM.BP_BOOOM_C" (Math|Transform|MakeTransform "-140.000000,-140.000000,110.000000") "Undefined" "MultiplyWithRoot" 0 0)
  (Game|SpawnActorfromClass "/Game/MyBP/BP_BOOOM.BP_BOOOM_C" (Math|Transform|MakeTransform "2870.000000,-160.000000,110.000000") "Undefined" "MultiplyWithRoot" 0 0)
  (Game|SpawnActorfromClass "/Game/MyBP/BP_BOOOM.BP_BOOOM_C" (Math|Transform|MakeTransform "2860.000000,2830.000000,110.000000") "Undefined" "MultiplyWithRoot" 0 0)
  (Utilities|FlowControl|Delay 1.0)
  (Rendering|SetVisibility (Variables|Default|GetParticleSystem) true false))

(event Collision|EventActorBeginOverlap
  (params (OtherActor :type Actor%20Object%20Reference)))

(event EventTick
  (params (DeltaSeconds :type Float%20%28single-precision%29)))

(fn ConstructionScript)