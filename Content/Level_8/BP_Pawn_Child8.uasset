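; Child pawn Blueprint for Level 8 that randomly changes the material on its Cube.
; After the parent BeginPlay and a short delay, a looping timer fires the RGB event every second.
; RGB uses nested random bools to apply one of three materials or leave the current one unchanged.
; A fourth material assignment is left disconnected, and the construction script only calls the parent.
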(event Custom|RGB
  (bind _cube (Variables|Default|GetCube))
  (if (Math|Random|RandomBool)
    (if (Math|Random|RandomBool)
      (Utilities|IsValid _cube
        (:Is%20Valid
          (Rendering|Material|SetMaterial _cube 0 "/Game/Level_5/NewMaterial3.NewMaterial3")))
      (else
        (Utilities|IsValid _cube
          (:Is%20Valid
            (Rendering|Material|SetMaterial _cube 0 "/Game/Level_5/NewMaterial5.NewMaterial5")))))
    (elif (Math|Random|RandomBool)
      (Utilities|IsValid (Variables|Default|GetCube)
        (:Is%20Valid
          (Rendering|Material|SetMaterial (Variables|Default|GetCube) 0 "/Game/Level_5/NewMaterial4.NewMaterial4"))))))

(event EventBeginPlay
  (|CallParentFunction)
  (Utilities|FlowControl|Delay 5.0)
  (Utilities|Time|SetTimerbyEvent (delegate Custom|RGB) 1.0 true))

(event Collision|EventActorBeginOverlap
  (params (OtherActor :type Actor%20Object%20Reference))
  (|CallParentFunction OtherActor) ; Этот узел отключен и не будет вызываться.\nПеретащите контакты, чтобы построить функционал.
)

(event EventTick
  (params (DeltaSeconds :type Float%20%28single-precision%29))
  (|CallParentFunction DeltaSeconds) ; Этот узел отключен и не будет вызываться.\nПеретащите контакты, чтобы построить функционал.
)

(fn ConstructionScript
  (|CallParentFunction))